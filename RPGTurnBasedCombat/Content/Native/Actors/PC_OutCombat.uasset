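; PC_OutCombat is the player controller for exploration outside combat, binding Enhanced Input for movement, attack and interaction.
; Attack plays an overhand montage, then sphere-traces forward; hitting an AI_Character sets PlayerShouldStart in GI_RPG and opens BaseCombatArea.
; Interact sphere-traces around the pawn and sends InteractMessage only after the hit loop completes, using its last element.
; Camera input is an empty event, with its look logic left disconnected.
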(event `self.ReceiveBeginPlay`
  (`EnhancedInputSubsystemInterface.AddMappingContext` (subsystem `EnhancedInputLocalPlayerSubsystem`) "/Game/Native/Input/IM_OutCombat.IM_OutCombat" 0 (struct)))

(event `EnhancedInput|/Game/Native/Input/IA_MoveOutCombat`
  (params (ActionValue :type "Vector2D Structure") (ElapsedSeconds :type "Float (double-precision)") (TriggeredSeconds :type "Float (double-precision)") (InputAction :type "InputAction Object Reference" :default "/Game/Native/Input/IA_MoveOutCombat.IA_MoveOutCombat"))
  (bind _returnvalue (`GameplayStatics.GetPlayerPawn` 0))
  (bind (_returnvalue_roll _returnvalue_pitch _returnvalue_yaw) (`KismetMathLibrary.BreakRotator` (`self.K2_GetActorRotation` _returnvalue)))
  (bind _returnvalue_2 (`KismetMathLibrary.MakeRotator` 0.0 0.0 _returnvalue_yaw))
  (:`Triggered`
    (`Pawn.AddMovementInput` _returnvalue (`KismetMathLibrary.GetForwardVector` _returnvalue_2) ActionValue_X false)
    (`Pawn.AddMovementInput` _returnvalue (`KismetMathLibrary.GetRightVector` _returnvalue_2) ActionValue_Y false)))

(event `EnhancedInput|/Game/Native/Input/IA_CameraOutCombat`
  (params (ActionValue :type "Vector2D Structure") (ElapsedSeconds :type "Float (double-precision)") (TriggeredSeconds :type "Float (double-precision)") (InputAction :type "InputAction Object Reference" :default "/Game/Native/Input/IA_CameraOutCombat.IA_CameraOutCombat")))

(event `EnhancedInput|/Game/Native/Input/IA_AttackOutCombat`
  (params (ActionValue :type Boolean) (ElapsedSeconds :type "Float (double-precision)") (TriggeredSeconds :type "Float (double-precision)") (InputAction :type "InputAction Object Reference" :default "/Game/Native/Input/IA_AttackOutCombat.IA_AttackOutCombat"))
  (:`Started`
    (if (`self.bCanAttack`)
      (set `self.bCanAttack` false)
      (bind _asout_combat_character (cast `/Game/Native/Actors/OutCombatCharacter` (`GameplayStatics.GetPlayerPawn` 0))
        (:`then`
          (`|PlayMontage` (`Character.Mesh` _asout_combat_character) "/Game/BoxingAttacks/TRADITIONAL/Attacks/KB_Overhand-R_T_Montage.KB_Overhand-R_T_Montage" 0.7
            (:`OnCompleted`
              (set `self.bCanAttack` true)
              (bind _returnvalue (`self.K2_GetActorLocation` _asout_combat_character))
              (bind _outhits (`KismetSystemLibrary.SphereTraceMulti` _returnvalue (+ _returnvalue (* (`self.GetActorForwardVector` _asout_combat_character) 150.0)) 100.0 "TraceTypeQuery2"))
              (for _array_element _outhits
                (cast `/Game/Native/Actors/AI_Character` (`.HitActor` (`GameplayStatics.BreakHitResult` _array_element)))
                (bind _asgi_rpg (cast `/Game/Native/Engine/GI_RPG` (`GameplayStatics.GetGameInstance`)))
                (set `/Game/Native/Engine/GI_RPG.bPlayerShouldStart` true _asgi_rpg)
                (`GameplayStatics.OpenLevelBySoftObjectPtr` "/Game/Level/BaseCombatArea.BaseCombatArea")))))
        (:`CastFailed`
          (set `self.bCanAttack` true))))))

(event `EnhancedInput|/Game/Native/Input/IA_InteractOutCombat`
  (params (ActionValue :type Boolean) (ElapsedSeconds :type "Float (double-precision)") (TriggeredSeconds :type "Float (double-precision)") (InputAction :type "InputAction Object Reference" :default "/Game/Native/Input/IA_InteractOutCombat.IA_InteractOutCombat"))
  (bind _returnvalue (`self.K2_GetActorLocation` (`GameplayStatics.GetPlayerPawn` 0)))
  (:`Started`
    (bind _outhits (`KismetSystemLibrary.SphereTraceMulti` _returnvalue _returnvalue 200.0 "TraceTypeQuery1"))
    (for _array_element _outhits
      _)
    (message `/Game/Native/Interact.Interact` (`.HitActor` (`GameplayStatics.BreakHitResult` _array_element)))))

(fn `UserConstructionScript`)