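; GM_RPG, apparently the RPG game mode, spawns and initializes the player team and groups of enemies.
; It caches the GI_RPG game instance on BeginPlay.
; GenerateRandomTeam spawns BP_BasePlayer actors without random stats despite its name, then stores the Team array in that game instance.
; GenerateRandomEnemies spawns a requested number of BP_BaseEnemy actors with random stats, appending them to Enemies and returning that array.
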(event `GenerateRandomTeam`
  (bind _rpggameinstance (`self.RPGGameInstance`))
  (for _ (range (`self.AmmountOfTeamMembers`))
    (bind _returnvalue (`|SpawnActorFromClass` "/Game/Shared/BP_BasePlayer.BP_BasePlayer_C" (`KismetMathLibrary.MakeTransform` (0.0 0.0 0.0)) "Undefined" "MultiplyWithRoot" null null))
    (`/Engine/EditorBlueprintResources/StandardMacros.IsValid` _returnvalue
      (:`Is Valid`
        (`BaseRPGCharacter.Init` _returnvalue false true)
        (`KismetArrayLibrary.Array_Add` (`self.Team`) _returnvalue))))
  (`/Engine/EditorBlueprintResources/StandardMacros.IsValid` _rpggameinstance
    (:`Is Valid`
      (set `/Game/Native/GI_RPG.Team` (`self.Team`) _rpggameinstance))))

(event `self.ReceiveBeginPlay`
  (bind _asgi_rpg (cast `/Game/Native/GI_RPG` (`GameplayStatics.GetGameInstance`)))
  (`/Engine/EditorBlueprintResources/StandardMacros.IsValid` _asgi_rpg
    (:`Is Valid`
      (set `self.RPGGameInstance` _asgi_rpg))))

(fn `GenerateRandomEnemies`
  (params (EnemiesAmmount :type Integer))
  (returns (GeneratedEnemies :type "Array of /Game/Shared/BP_BaseEnemy Object Reference"))
  (locals (Enemies :type "Array of /Game/Shared/BP_BaseEnemy Object Reference"))
  (bind _enemies (`local.Enemies`))
  (for _ (range EnemiesAmmount)
    (bind _returnvalue (`|SpawnActorFromClass` "/Game/Shared/BP_BaseEnemy.BP_BaseEnemy_C" (`KismetMathLibrary.MakeTransform` (0.0 0.0 0.0)) "Undefined" "MultiplyWithRoot" null null))
    (`/Engine/EditorBlueprintResources/StandardMacros.IsValid` _returnvalue
      (:`Is Valid`
        (`BaseRPGCharacter.Init` _returnvalue true false)
        (`KismetArrayLibrary.Array_Add` _enemies _returnvalue))))
  (return _enemies))

(fn `UserConstructionScript`)